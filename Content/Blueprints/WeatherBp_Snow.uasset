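; Weather Blueprint that toggles snowy weather with the T key, as long as the Sky reference is valid.
; A FlipFlop starts a timeline that blends the sky material's zenith, horizon and cloud colors, cloud opacity and light color toward overcast grey, then activates the snow particles after a delay.
; The next press stops the particles, waits briefly, then reverses the timeline to restore the clear sky.
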(event `Key|T`
  (params (Key :type "Key Structure"))
  (bind _sky_material (`/Engine/EngineSky/BP_Sky_Sphere.Sky material` (`self.Sky`)))
  (bind _particlesystemcomponent (`Emitter.ParticleSystemComponent` (`self.Snow ref`)))
  ;[1 1 1] Snow
  (:`Pressed`
    (if (`KismetSystemLibrary.IsValid` (`self.Sky`))
      (`/Engine/EditorBlueprintResources/StandardMacros.FlipFlop`
        (:`A`
          (`|ExecutionSequence`
            (:`then_0`
              (bind (_direction _newtrack_1) (`Timeline|Timeline_1` :!label _label)
                (:`Update`
                  (`MaterialInstanceDynamic.SetVectorParameterValue` _sky_material "Zenith Color" (`KismetMathLibrary.LinearColorLerp` (struct :`R` 0.034046 :`G` 0.109247 :`B` 0.295 :`A` 1.0) (struct :`R` 0.359375 :`G` 0.359375 :`B` 0.359375 :`A` 1.0) _newtrack_1))
                  (`MaterialInstanceDynamic.SetVectorParameterValue` _sky_material "Horizon Color" (`KismetMathLibrary.LinearColorLerp` (struct :`R` 1.979559 :`G` 2.586644 :`B` 3.0 :`A` 1.0) (struct :`R` 0.390625 :`G` 0.390625 :`B` 0.390625 :`A` 1.0) _newtrack_1))
                  (`MaterialInstanceDynamic.SetVectorParameterValue` _sky_material "Cloud Color" (`KismetMathLibrary.LinearColorLerp` (struct :`R` 0.855778 :`G` 0.91902 :`B` 1.0 :`A` 1.0) (struct :`R` 0.401042 :`G` 0.401042 :`B` 0.401042 :`A` 1.0) _newtrack_1))
                  (`MaterialInstanceDynamic.SetScalarParameterValue` _sky_material "Cloud Opacity" (`KismetMathLibrary.Lerp` 1.0 5.0 _newtrack_1))
                  (`LightComponent.SetLightColor` (`Light.LightComponent` (`self.light`)) (`KismetMathLibrary.LinearColorLerp` (struct :`R` 0.855778 :`G` 0.91902 :`B` 1.0 :`A` 1.0) (struct :`R` 0.333333 :`G` 0.333333 :`B` 0.333333 :`A` 1.0) _newtrack_1) true))))
            (:`then_1`
              (`KismetSystemLibrary.Delay` 5.0)
              (`ActorComponent.Activate` _particlesystemcomponent false))))
        (:`B`
          (`ActorComponent.Deactivate` _particlesystemcomponent)
          (`KismetSystemLibrary.Delay` 3.0)
          (goto _label :!via `Reverse`))))))

(fn `UserConstructionScript`)